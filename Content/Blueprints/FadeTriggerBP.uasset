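; Trigger actor that handles screen fades through a FadeWidget, including a fade-out that restarts the current level.
; BeginPlay and FirstPersonCharacter overlap on its Box share one chain that creates the widget, adds it to the viewport, destroys the actor and calls FadeIn.
; TriggerFade calls FadeOff on the stored widget, waits through a Delay and reopens the current level by name.
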(event OnComponentBeginOverlap(Box)
  (params (OverlappedComponent :type Primitive%20Component%20Object%20Reference) (OtherActor :type Actor%20Object%20Reference) (OtherComp :type Primitive%20Component%20Object%20Reference) (OtherBodyIndex :type Integer) (bFromSweep :type Boolean) (SweepResult :type Hit%20Result%20Structure%20%28by%20ref%29))
  ;[1 1 1] Fade In
  (Utilities|Casting|CastToFirstPersonCharacter OtherActor)
  (Utilities|FlowControl|Sequence
    (:then_0
      (bind _returnvalue (UserInterface|CreateWidget "/Game/Widgets/FadeWidget.FadeWidget_C" (Game|GetPlayerController 0)))
      (bind _asfade_widget (Utilities|Casting|CastToFadeWidget _returnvalue))
      (Variables|Default|SetAs%20Fade%20Widget _asfade_widget)
      (UserInterface|Viewport|AddtoViewport _returnvalue 0)
      (Actor|DestroyActor))
    (:then_1
      (Default|Fadein (Variables|Default|GetAs%20Fade%20Widget)))))

(event Custom|TriggerFade
  ;[1 1 1] Fade Out
  (Default|FadeOff (Variables|Default|GetAs%20Fade%20Widget))
  (Utilities|FlowControl|Delay 4.0)
  (bind _returnvalue (Game|GetCurrentLevelName true))
  (Game|OpenLevel(byName) (Utilities|String|StringToName _returnvalue)))

(event EventBeginPlay
  ;[1 1 1] Fade In
  (Utilities|FlowControl|Sequence
    (:then_0
      (bind _returnvalue (UserInterface|CreateWidget "/Game/Widgets/FadeWidget.FadeWidget_C" (Game|GetPlayerController 0)))
      (bind _asfade_widget (Utilities|Casting|CastToFadeWidget _returnvalue))
      (Variables|Default|SetAs%20Fade%20Widget _asfade_widget)
      (UserInterface|Viewport|AddtoViewport _returnvalue 0)
      (Actor|DestroyActor))
    (:then_1
      (Default|Fadein (Variables|Default|GetAs%20Fade%20Widget)))))

(fn ConstructionScript)