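; Pickup key for the art room that the player collects by walking into it.
; On overlap with the player character, it increments the character's KeyArtRoom count and prints it.
; It then calls UnhideEnemy on its referenced Enemy to make that enemy appear, and destroys itself.
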(event OnComponentBeginOverlap(Collision)
  (params (OverlappedComponent :type Primitive%20Component%20Object%20Reference) (OtherActor :type Actor%20Object%20Reference) (OtherComp :type Primitive%20Component%20Object%20Reference) (OtherBodyIndex :type Integer) (bFromSweep :type Boolean) (SweepResult :type Hit%20Result%20Structure%20%28by%20ref%29))
  (bind _returnvalue (Game|GetPlayerCharacter 0))
  ;[1 1 1] Key
  (if (== OtherActor _returnvalue)
    (bind _asfirst_person_character (Utilities|Casting|CastToFirstPersonCharacter _returnvalue))
    (bind _result (Math|Integer|IncrementInt (Variables|/Game/FirstPersonBP/Blueprints/FirstPersonCharacter.FirstPersonCharacter_C|GetKeyArtRoom _asfirst_person_character))
      (:%20%20
        (Development|PrintString (Utilities|String|ToString(Integer) _result) true true "(R=0.052749,G=1.000000,B=0.000000,A=1.000000)")
        ;;[1 1 1] Makes Enemy Appear
        (bind _asenemy (Utilities|Casting|CastToEnemy (Variables|Default|GetEnemy)))
        (Default|UnhideEnemy _asenemy)
        (Actor|DestroyActor self)))))

(fn ConstructionScript)