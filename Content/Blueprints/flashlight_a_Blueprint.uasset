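; Flashlight pickup actor that grants the player a flashlight when they overlap its sphere.
; The overlap sets HaveFlashLight on FirstPersonCharacter, then shows an existing interaction widget or creates one with InteractionText.
; Only the creation branch hides the mesh, waits briefly, hides the widget and destroys the actor.
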(event OnComponentBeginOverlap(Sphere)
  (params (OverlappedComponent :type Primitive%20Component%20Object%20Reference) (OtherActor :type Actor%20Object%20Reference) (OtherComp :type Primitive%20Component%20Object%20Reference) (OtherBodyIndex :type Integer) (bFromSweep :type Boolean) (SweepResult :type Hit%20Result%20Structure%20%28by%20ref%29))
  (bind _returnvalue (Game|GetPlayerCharacter 0))
  ;[1 1 1] Pickup Destroy
  (if (== OtherActor _returnvalue)
    (bind _asfirst_person_character (Utilities|Casting|CastToFirstPersonCharacter _returnvalue))
    (Variables|/Game/FirstPersonBP/Blueprints/FirstPersonCharacter.FirstPersonCharacter_C|SetHaveFlashLight? _asfirst_person_character true)
    (Utilities|IsValid (Variables|Default|GetWidget)
      (:Is%20Valid
        (Widget|SetVisibility (Variables|Default|GetWidget) "Visible"))
      (:Is%20Not%20Valid
        (bind _returnvalue_2 (UserInterface|CreateWidget "/Game/Widgets/InteractionWidget.InteractionWidget_C"))
        (Variables|/Game/Widgets/InteractionWidget.InteractionWidget_C|SetInteractionText _returnvalue_2 (Variables|Default|GetInteraction%20Text))
        (bind _output_get (Variables|Default|SetWidget _returnvalue_2))
        (UserInterface|Viewport|AddtoViewport _output_get 0)
        (Rendering|SetVisibility (Variables|Debug|GetStaticMeshComponent) false true)
        (Utilities|FlowControl|Delay 1.0)
        (Widget|SetVisibility (Variables|Default|GetWidget) "Hidden")
        (Actor|DestroyActor self)))))

(fn ConstructionScript)