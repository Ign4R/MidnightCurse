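; Enemy Blueprint that chases the player character after a configurable start delay.
; On BeginPlay it caches the player reference, then loops AI MoveTo toward the player, retrying 0.2 seconds after each success or failure while Chase is true.
; Any overlap with its capsule component sets Chase to false, ending the loop at its next check.
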(event OnComponentBeginOverlap(CapsuleComponent)
  (params (OverlappedComponent :type Primitive%20Component%20Object%20Reference) (OtherActor :type Actor%20Object%20Reference) (OtherComp :type Primitive%20Component%20Object%20Reference) (OtherBodyIndex :type Integer) (bFromSweep :type Boolean) (SweepResult :type Hit%20Result%20Structure%20%28by%20ref%29))
  (Variables|Default|Setchase false))

(event EventBeginPlay
  ;[1 1 1] Get Player Reference
  (Variables|Default|Setplayer_ref (Game|GetPlayerCharacter 0))
  ;[1 1 1] Time to start chasing player
  (Utilities|FlowControl|Delay (Variables|Default|GetstartChase))
  ;[1 1 1] Chase Condition
  (if (Variables|Default|Getchase) :!label _label
    ;[1 1 1] Move AI
    (AI|AIMoveTo self (Transformation|GetActorLocation (Variables|Default|Getplayer_ref)) (Variables|Default|Getplayer_ref) 5.0 false
      (:OnSuccess
        _)
      (:OnFail
        _))
    ;[1 1 1] Loop
    (Utilities|FlowControl|Delay 0.2)
    (goto _label)))

(fn ConstructionScript)