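; Child room door Blueprint that swings open when the player overlaps its trigger while holding a ChildRoom key, and otherwise prints a warning.
; The overlap event casts the player to FirstPersonCharacter, checks KeyChildRoom, then calls TakeKey and OpenDoor.
; OpenDoor plays a timeline that lerps Door3 from its BeginPlay rotation to a fixed open rotation.
; TakeKey only caps the key count at one, so the key is never consumed.
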(event OnComponentBeginOverlap(Overlap)
  (params (OverlappedComponent :type Primitive%20Component%20Object%20Reference) (OtherActor :type Actor%20Object%20Reference) (OtherComp :type Primitive%20Component%20Object%20Reference) (OtherBodyIndex :type Integer) (bFromSweep :type Boolean) (SweepResult :type Hit%20Result%20Structure%20%28by%20ref%29))
  ;[1 1 1] Open Door
  (if (== OtherActor (Game|GetPlayerCharacter 0)) ; Overlap with Player
    (bind _asfirst_person_character (Utilities|Casting|CastToFirstPersonCharacter (Game|GetPlayerCharacter 0))) ; Get Player
    (bind _output_get (Variables|Default|SetAs%20First%20Person%20Character _asfirst_person_character))
    (if (> (Variables|/Game/FirstPersonBP/Blueprints/FirstPersonCharacter.FirstPersonCharacter_C|GetKeyChildRoom _output_get) 0) ; Does player has key?
      (|TakeKey) ; Take key
      (CallFunction|OpenDoor)
      (else
        (Development|PrintString "You need ChildRoom key!" true true "(R=1.000000,G=0.000000,B=0.955812,A=1.000000)")))))

(event Custom|Open%20Door
  ;[1 1 1] Open Door
  (bind _0_to_1 (Timeline|0%20to%201 Play)
    (:Update
      (Transformation|SetRelativeRotation (Variables|Default|GetDoor3) (Math|Rotator|Lerp(Rotator) (Variables|Default|GetDoor3Origin) "0,90.000000, 0" _0_to_1 true) false false))))

(event EventBeginPlay
  ;[1 1 1] Open Door
  (Variables|Default|SetDoor3Origin (Variables|/Script/Engine.SceneComponent|GetRelativeRotation (Variables|Default|GetDoor3))))

(fn ConstructionScript)