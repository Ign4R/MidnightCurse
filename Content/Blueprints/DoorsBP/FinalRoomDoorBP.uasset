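; Final room door Blueprint that opens when the player enters its overlap volume holding a child room key.
; The overlap checks the player character's KeyChildRoom count, then TakeKey caps it at one and OpenDoor plays a timeline lerping the door from its starting rotation.
; Without a key, it shows an interaction text widget, created once and reused, which hides when an actor's overlap ends.
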(event OnComponentBeginOverlap(Overlap)
  (params (OverlappedComponent :type Primitive%20Component%20Object%20Reference) (OtherActor :type Actor%20Object%20Reference) (OtherComp :type Primitive%20Component%20Object%20Reference) (OtherBodyIndex :type Integer) (bFromSweep :type Boolean) (SweepResult :type Hit%20Result%20Structure%20%28by%20ref%29))
  ;[1 1 1] Open Door
  (if (== OtherActor (Game|GetPlayerCharacter 0)) ; Overlap with Player
    (bind _asfirst_person_character (Utilities|Casting|CastToFirstPersonCharacter (Game|GetPlayerCharacter 0))) ; Get Player
    (bind _output_get (Variables|Default|SetAs%20First%20Person%20Character _asfirst_person_character))
    (if (> (Variables|/Game/FirstPersonBP/Blueprints/FirstPersonCharacter.FirstPersonCharacter_C|GetKeyChildRoom _output_get) 0) ; Does player has key?
      (|TakeKey) ; Take key
      (CallFunction|OpenDoor)
      (else
        (Utilities|IsValid (Variables|Default|GetWidget)
          (:Is%20Valid
            (Widget|SetVisibility (Variables|Default|GetWidget) "Visible"))
          (:Is%20Not%20Valid
            (bind _returnvalue (UserInterface|CreateWidget "/Game/Widgets/InteractionWidget.InteractionWidget_C"))
            (Variables|/Game/Widgets/InteractionWidget.InteractionWidget_C|SetInteractionText _returnvalue (Variables|Default|GetInteraction%20Text%20))
            (bind _output_get_2 (Variables|Default|SetWidget _returnvalue))
            (UserInterface|Viewport|AddtoViewport _output_get_2 0)))))))

(event Custom|Open%20Door
  ;[1 1 1] Animation door
  (bind _0_to_1 (Timeline|0%20to%201 Play)
    (:Update
      (Transformation|SetRelativeRotation (Variables|Default|GetDoor) (Math|Rotator|Lerp(Rotator) (Variables|Default|GetDoor3Origin) "0,90.000000, 0" _0_to_1 true) false false))))

(event Collision|EventActorEndOverlap
  (params (OtherActor :type Actor%20Object%20Reference))
  (bind _widget (Variables|Default|GetWidget))
  ;[1 1 1] Open Door
  (Utilities|IsValid _widget
    (:Is%20Valid
      (Widget|SetVisibility _widget "Hidden"))))

(event EventBeginPlay
  ;[1 1 1] Animation door
  (Variables|Default|SetDoor3Origin (Variables|/Script/Engine.SceneComponent|GetRelativeRotation (Variables|Default|GetDoor))))

(fn ConstructionScript)