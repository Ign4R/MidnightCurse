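; Bookshelf actor that plays a one-time jumpscare when the first-person character enters its trigger volume.
; The overlap turns on physics for two book components, pushes them along world Y and plays the jumpscare sound at the actor's location.
; It then destroys the trigger so the scare cannot repeat, and removes both books after a short delay.
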(event OnComponentBeginOverlap(Trigger)
  (params (OverlappedComponent :type Primitive%20Component%20Object%20Reference) (OtherActor :type Actor%20Object%20Reference) (OtherComp :type Primitive%20Component%20Object%20Reference) (OtherBodyIndex :type Integer) (bFromSweep :type Boolean) (SweepResult :type Hit%20Result%20Structure%20%28by%20ref%29))
  (bind _bookjumpscare1 (Variables|Default|GetBookJumpscare1))
  ;[1 1 1] Bookshelf
  (Utilities|Casting|CastToFirstPersonCharacter OtherActor)
  (Physics|SetSimulatePhysics _bookjumpscare1 true)
  (Physics|AddForce _bookjumpscare1 "0,250.000000, 0" "None" false)
  (Audio|PlaySoundatLocation "/Game/MyAudios/Jumpscare_Sound_Effect.Jumpscare_Sound_Effect" (Transformation|GetActorLocation) "0, 0, 0" 1.0 1.0 0.0 0 0 0)
  (Components|DestroyComponent (Variables|Default|GetTrigger))
  (Utilities|FlowControl|Delay 5.0)
  (Components|DestroyComponent (Variables|Default|GetBookJumpscare)))

(fn ConstructionScript)